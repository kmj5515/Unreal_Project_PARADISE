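; Player controller for the main menu that brings up the menu UI when play begins.
; It first adds a fade-out widget to the viewport, then waits through a fixed delay.
; It then shows the mouse cursor, adds the main menu widget and switches input to UI-only mode focused on that menu.
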(event `self.ReceiveBeginPlay`
  (bind _returnvalue (`|CreateWidget` "/Game/Horror_Template/UI/Main_Menu_UI/WBP_Fade_OUT_Main_Menu.WBP_Fade_OUT_Main_Menu_C"))
  (bind _output_get (set `self.Fade Out UI` _returnvalue))
  (`UserWidget.AddToViewport` _output_get 0)
  (`KismetSystemLibrary.Delay` 5.0)
  (set `self.bShowMouseCursor` true)
  (bind _returnvalue_2 (`|CreateWidget` "/Game/Horror_Template/UI/Main_Menu_UI/WBP_Main_Menu.WBP_Main_Menu_C"))
  (bind _output_get_2 (set `self.Main Menu UI` _returnvalue_2))
  (`UserWidget.AddToViewport` _output_get_2 0)
  (`WidgetBlueprintLibrary.SetInputMode_UIOnlyEx` self (`self.Main Menu UI`)))

(fn `UserConstructionScript`)